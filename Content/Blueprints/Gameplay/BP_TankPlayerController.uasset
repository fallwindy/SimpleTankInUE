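; Player controller for the tank game that owns the HUD and decides when the match is won or lost.
; It creates crosshair, health and minimap widgets, then polls every Tick.
; The crosshair follows the screen projection of FireTraceHit, highlighting hit Pawns and hiding without a hit.
; Tank health and remaining BP_EnemyTank count feed the health widget; zero enemies or a dead player triggers a delayed pause and win/lose screen.
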(event `self.ReceiveBeginPlay`
  (bind _returnvalue (`|CreateWidget` "/Game/Blueprints/UI/UI_Crosshair.UI_Crosshair_C"))
  (bind _output_get (set `self.Crosshair` _returnvalue))
  (`UserWidget.AddToViewport` _output_get 0)
  (bind _returnvalue_2 (`|CreateWidget` "/Game/Blueprints/UI/UI_MyHealth.UI_MyHealth_C"))
  (bind _output_get_2 (set `self.PlayerHealthUI` _returnvalue_2))
  (`UserWidget.AddToViewport` _output_get_2 0)
  (bind _returnvalue_3 (`|CreateWidget` "/Game/Blueprints/UI/UI_MiniMap.UI_MiniMap_C"))
  (`UserWidget.AddToViewport` _returnvalue_3 0))

(event `self.ReceiveTick`
  (params (DeltaSeconds :type "Float (single-precision)"))
  (`self.UpdateCrosshairUI`)
  (`self.UpdatePlayerHealth`)
  (`self.UpdateEnemys`))

(event `UpdateEnemys`
  (bind _outactors (`GameplayStatics.GetAllActorsOfClass` "/Game/Blueprints/Enemy/BP_EnemyTank.BP_EnemyTank_C"))
  (bind _returnvalue (`KismetArrayLibrary.Array_Length` _outactors))
  (`/Game/Blueprints/UI/UI_MyHealth.SetEnemyNums` (`self.PlayerHealthUI`) _returnvalue)
  (if (and (== _returnvalue 0) (`KismetSystemLibrary.IsValid` (`GameplayStatics.GetPlayerPawn` 0)))
    (`self.EndUI`
      (:`then`)
      (:`else`
        (`KismetSystemLibrary.Delay` 5.0)
        (`GameplayStatics.SetGamePaused` true)
        (bind _returnvalue_2 (`|CreateWidget` "/Game/Blueprints/UI/UI_GameEnding.UI_GameEnding_C" null "你赢了"))
        (`UserWidget.AddToViewport` _returnvalue_2 0)
        (set `self.EndUI` _returnvalue_2)
        (set `self.bShowMouseCursor` true)))))

(event `UpdatePlayerHealth`
  (bind _returnvalue (`self.K2_GetPawn`))
  (bind _asbp_my_tank (cast `/Game/Blueprints/Pawns/BP_MyTank` _returnvalue :!pure true))
  (bind _returnvalue_2 (/ (`MyTankBase.CurHealth` _asbp_my_tank) (`MyTankBase.MaxHealth` _asbp_my_tank)))
  (`/Engine/EditorBlueprintResources/StandardMacros.IsValid` _returnvalue
    (:`Is Valid`
      (bind _playerhealthui (`self.PlayerHealthUI`)
        (:`then`
          (`/Game/Blueprints/UI/UI_MyHealth.SetHealthPercent` _playerhealthui _returnvalue_2)
          (if (<= _returnvalue_2 0.0)
            (`self.EndUI` :!label _label
              (:`then`)
              (:`else`
                (`KismetSystemLibrary.Delay` 5.0)
                (`GameplayStatics.SetGamePaused` true)
                (bind _returnvalue_3 (`|CreateWidget` "/Game/Blueprints/UI/UI_GameEnding.UI_GameEnding_C" null "你输了"))
                (`UserWidget.AddToViewport` _returnvalue_3 0)
                (set `self.EndUI` _returnvalue_3)
                (set `self.bShowMouseCursor` true)))))
        (:`else`)))
    (:`Is Not Valid`
      (`/Game/Blueprints/UI/UI_MyHealth.SetHealthPercent` (`self.PlayerHealthUI`) 0.0)
      (goto _label))))

(fn `UpdateCrosshairUI`
  (bind _crosshair (`self.Crosshair`))
  (bind (_bblockinghit _binitialoverlap _time _distance _location _impactpoint _normal _impactnormal _physmat _hitactor) (`GameplayStatics.BreakHitResult` (`self.FireTraceHit`)))
  (bind (_x _y) (`KismetMathLibrary.BreakVector2D` (`self.ProjectWorldLocationToScreen` _location)))
  (if _bblockinghit
    (`Widget.SetVisibility` (`self.Crosshair`) "Visible")
    (`UserWidget.SetPositionInViewport` _crosshair (`KismetMathLibrary.MakeVector2D` (+ _x -20.0) (+ _y -20.0)) true)
    (cast `Pawn` _hitactor
      (:`then`
        (`UserWidget.SetColorAndOpacity` _crosshair (struct :`R` 0.911458 :`G` 0.002773 :`B` 0.166947 :`A` 1.0))
        (`Widget.SetRenderScale` _crosshair (1.1 1.1))
        (`Widget.SetRenderScale` (`self.Crosshair`) (1.1 1.1)))
      (:`CastFailed`
        (`UserWidget.SetColorAndOpacity` _crosshair (struct :`R` 1.0 :`G` 1.0 :`B` 1.0 :`A` 1.0))
        (`Widget.SetRenderScale` (`self.Crosshair`) (1.0 1.0))))
    (else
      (`Widget.SetVisibility` (`self.Crosshair`) "Hidden"))))

(fn `UserConstructionScript`)