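; Base tank pawn with tracked steering, gun elevation input and death handling.
; Each tick, throttle and steering become left and right track inputs for BPTankMoveComponent: straight, opposed for turning in place, or throttle on one track for moving turns.
; An input axis adjusts a clamped gun elevation value.
; The damage event swaps the tank for a BP_DamgedTank actor once health is depleted.
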(event `self.ReceiveTick`
  (params (DeltaSeconds :type "Float (single-precision)"))
  (`self.UpdateInput`))

(event `InputAxis|AdjustGunElevation`
  (params (AxisValue :type "Float (single-precision)"))
  (set `self.GunElevation` (`KismetMathLibrary.FClamp` (- (`self.GunElevation`) AxisValue) -15.0 15.0)))

(event `self.BPDamage`
  (if (<= (`self.CurHealth`) 0.0)
    (`|SpawnActorFromClass` "/Game/Blueprints/BP_DamgedTank.BP_DamgedTank_C" (`self.GetTransform`) "Undefined" "OverrideRootScale" null null)
    (`self.K2_DestroyActor`)))

(fn `UpdateInput`
  (locals (LeftInput :type "Float (double-precision)" :default 0.0) (RightInput :type "Float (double-precision)" :default 0.0))
  (bind _throttle (`self.Throttle`))
  (bind _steering (`self.Steering`))
  (set `self.Throttle` (`self.GetInputAxisValue`))
  (set `self.Steering` (`self.GetInputAxisValue`))
  (`|ExecutionSequence`
    (:`then_0`
      (if (xor (!= (`self.Throttle`) 0.0) (!= (`self.Steering`) 0.0))
        (if (!= (`self.Throttle`) 0.0)
          (set `local.LeftInput` _throttle)
          (set `local.RightInput` _throttle)
          (else
            (set `local.LeftInput` _steering)
            (set `local.RightInput` (* -1 _steering))))
        (elif (!= (`self.Throttle`) 0.0)
          (if (> (`self.Steering`) 0.0)
            (set `local.LeftInput` (`self.Throttle`))
            (else
              (set `local.RightInput` (`self.Throttle`)))))))
    (:`then_1`
      (`TankMoveComponent.SetMovementInput` (`self.BP_TankMoveComponent`) (`local.LeftInput`) (`local.RightInput`)))))

(fn `UserConstructionScript`
  (`PrimitiveComponent.CreateDynamicMaterialInstance` (`self.Mesh`) 1 null "None"))