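; BP_MyTank is a tank pawn that adds a reload indicator and an aim view.
; It creates a UI_Reload widget on BeginPlay and removes it on destruction.
; Each tick, while ReckonTime is below ReloadTime, the widget follows the tank's projected screen position and shows circular progress.
; Holding AimAt spawns a narrow-FOV BP_Aim_Camera at the gun socket and switches view to it, restoring it on release.
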(event `self.ReceiveBeginPlay`
  (`parent.ReceiveBeginPlay`)
  (bind _returnvalue (`|CreateWidget` "/Game/Blueprints/UI/UI_Reload.UI_Reload_C"))
  (bind _output_get (set `self.ReloadUI` _returnvalue))
  (`UserWidget.AddToViewport` _output_get 0))

(event `self.ReceiveTick`
  (params (DeltaSeconds :type "Float (single-precision)"))
  (`parent.ReceiveTick` DeltaSeconds)
  (`self.UpdateReloadUI`))

(event `self.ReceiveDestroyed`
  (`Widget.RemoveFromParent` (`self.ReloadUI`)))

(event `InputAction|AimAt`
  (params (Key :type "Key Structure"))
  (:`Pressed`
    (bind _returnvalue (`|SpawnActorFromClass` "/Game/Blueprints/BP_Aim_Camera.BP_Aim_Camera_C" (`SceneComponent.GetSocketTransform` (`self.Mesh`) "gun_1_jntSocket" "RTS_World") "Undefined" "OverrideRootScale" null null))
    (`PlayerController.SetViewTargetWithBlend` (`GameplayStatics.GetPlayerController` 0) _returnvalue 0.0 "VTBlend_Linear" 0.0 false)
    (`CameraComponent.SetFieldOfView` (`/Game/Blueprints/BP_Aim_Camera.Camera` _returnvalue) 20.0))
  (:`Released`
    (`PlayerController.SetViewTargetWithBlend` (`GameplayStatics.GetPlayerController` 0) self 0.0 "VTBlend_Linear" 0.0 false)
    (`self.K2_DestroyActor` _returnvalue)))

(fn `UpdateReloadUI`
  (bind _reloadui (`self.ReloadUI`))
  (if (< (`self.ReckonTime`) (`self.ReloadTime`))
    (`Widget.SetVisibility` _reloadui "Visible")
    (`UserWidget.SetPositionInViewport` _reloadui (`PlayerController.ProjectWorldLocationToScreen` (`GameplayStatics.GetPlayerController` 0) (`self.K2_GetActorLocation`) false) true)
    (`/Game/Blueprints/UI/UI_Reload.SetCirclePercent` _reloadui (/ (`self.ReckonTime`) (`self.ReloadTime`)))
    (else
      (`Widget.SetVisibility` (`self.ReloadUI`) "Hidden"))))

(fn `UserConstructionScript`
  (`parent.UserConstructionScript`))