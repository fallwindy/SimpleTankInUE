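; AI controller for enemy tanks that targets and fires on BP_MyTank.
; On BeginPlay it runs Enemy_AITree and caches the controlled BP_EnemyTank.
; Each tick a large debug-drawn sphere trace around the tank looks for pawns, ignoring all enemy tanks via a per-frame GetAllActorsOfClass.
; A BP_MyTank hit sets control rotation and GunRotation toward it, then calls Fire every tick without any cooldown here.
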(event `self.ReceiveBeginPlay`
  (`self.RunBehaviorTree` "/Game/Blueprints/Enemy/Enemy_AITree.Enemy_AITree")
  (bind _asbp_enemy_tank (cast `/Game/Blueprints/Enemy/BP_EnemyTank` (`self.K2_GetPawn`)))
  (set `self.ControlledEnemy Tank` _asbp_enemy_tank))

(event `self.ReceiveTick`
  (params (DeltaSeconds :type "Float (single-precision)"))
  (bind _returnvalue (`self.K2_GetActorLocation` (`self.ControlledEnemy Tank`)))
  (bind _outactors (`GameplayStatics.GetAllActorsOfClass` "/Game/Blueprints/Enemy/BP_EnemyTank.BP_EnemyTank_C"))
  (bind _outhit (`KismetSystemLibrary.SphereTraceSingleForObjects` _returnvalue _returnvalue 15000.0 (`|MakeArray` "ObjectTypeQuery3" :!type "EObjectTypeQuery Enum") false _outactors "ForOneFrame"))
  (bind _asbp_my_tank (cast `/Game/Blueprints/Pawns/BP_MyTank` (`.HitActor` (`GameplayStatics.BreakHitResult` _outhit))))
  (bind _returnvalue_2 (`KismetMathLibrary.MakeRotFromX` (- (`self.K2_GetActorLocation` _asbp_my_tank) (`self.K2_GetActorLocation` (`self.ControlledEnemy Tank`)))))
  (`self.SetControlRotation` _returnvalue_2)
  (set `self.GunRotation` _returnvalue_2)
  (`MyTankBase.Fire` (`self.ControlledEnemy Tank`)))

(fn `UserConstructionScript`)